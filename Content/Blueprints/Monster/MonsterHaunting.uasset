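; Haunting monster that appears at a random map location with a droning sound and glides toward the player at a fixed height.
; BeginPlay starts HauntLoop, while Tick holds off pursuit for a random initial delay via SpawnCheck.
; When its projected position is within the viewport and the player is near, it hides Norrman with a poof sound, silences the drone and reruns HauntLoop minutes later.
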(event Custom|HauntLoop
  (bind _droning (Variables|Default|GetDroning))
  (if (Audio|Components|Audio|IsPlaying _droning)
    _
    (else
      (Audio|Components|Audio|Play _droning 0.0)))
  (Transformation|SetActorLocation (Math|Vector|MakeVector (Math|Random|RandomFloatinRange -25433.0 18244.0) (Math|Random|RandomFloatinRange -26244.0 18061.0) 4e+02) false false)
  (Rendering|SetVisibility (Variables|Default|Getnorrman) true false))

(event EventBeginPlay
  (Components|Timeline|SetLooping (Variables|Default|GetFloofsPoof) false)
  (CallFunction|HauntLoop))

(event EventTick
  (params (DeltaSeconds :type Float%20%28single-precision%29))
  (bind _returnvalue (Transformation|GetActorLocation))
  (bind _returnvalue_2 (Game|GetPlayerController 0))
  (bind _returnvalue_3 (Transformation|GetActorLocation))
  (bind _returnvalue_4 (Viewport|GetViewportSize))
  (bind _returnvalue_5 (Game|GetPlayerCharacter 0))
  (bind _returnvalue_6 (Transformation|GetActorLocation _returnvalue_5))
  (bind _screenlocation (Class|PlayerController|ProjectWorldLocationtoScreen _returnvalue_2 _returnvalue_3 false))
  (bind _returnvalue_7 (- _returnvalue_6 _returnvalue))
  (bind _returnvalue_8 (Math|Vector|Normalize _returnvalue_7))
  (bind _returnvalue_9 (* _returnvalue_8 DeltaSeconds))
  (bind _returnvalue_10 (* _returnvalue_9 3e+02))
  (bind _returnvalue_11 (+ _returnvalue _returnvalue_10))
  (if (< (stale _output_get) 1)
    (bind _output_get (Variables|Default|SetSpawnCheck (stale _result)))
    (Utilities|FlowControl|Delay (Math|Random|RandomFloatinRange 6e+01 1.8e+02))
    (bind _result (Math|Integer|IncrementInt (Variables|Default|GetSpawnCheck)))
    (else
      (if (Math|Boolean|ANDBoolean (> (.x _screenlocation) 0.0) (> (.y _screenlocation) 0.0) (< (.x _screenlocation) (.x _returnvalue_4)) (< (.y _screenlocation) (.y _returnvalue_4)) (< (Transformation|GetDistanceTo _returnvalue_5 (Components|GetOwner (Variables|Default|Getnorrman))) 2e+03))
        (Rendering|SetVisibility (Variables|Default|Getnorrman) false false)
        (Audio|Components|Audio|Play (Variables|Default|GetFloofsPoof))
        (Audio|Components|Audio|Stop (Variables|Default|GetDroning))
        (Utilities|FlowControl|Delay (Math|Random|RandomFloatinRange 1.8e+02 4.2e+02))
        (CallFunction|HauntLoop))
      (Transformation|SetActorLocation (Math|Vector|MakeVector (.x _returnvalue_11) (.y _returnvalue_11) 4e+02) false false))))

(fn ConstructionScript)