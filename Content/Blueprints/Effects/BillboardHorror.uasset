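; BillboardHorror is an effect Blueprint that signals when the player character turns quickly.
; BeginPlay caches the player and its forward vector, then Tick dots the previous vector with the current one flattened to XY.
; When that dot product, multiplied by DeltaSeconds, falls below TurnDotTreshold, it calls the OnPlayerTurnedQuickly dispatcher.
; The flattened forward vector is then stored for the next frame.
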(event EventBeginPlay
  (bind _output_get (Variables|Default|SetPlayer (Game|GetPlayerCharacter 0)))
  (Variables|Default|SetPrevLookat (Transformation|GetActorForwardVector _output_get)))

(event EventTick
  (params (DeltaSeconds :type Float%20%28single-precision%29))
  (bind _player (Variables|Default|GetPlayer))
  (bind _returnvalue (Transformation|GetActorForwardVector _player))
  (bind (_x _y) (Math|Vector|BreakVector _returnvalue))
  (bind _returnvalue_2 (Math|Vector|MakeVector _x _y 0.0))
  (Utilities|FlowControl|Sequence
    (:then_0
      (if (> (Variables|Default|GetTurnDotTreshold) (* DeltaSeconds (Math|Vector|DotProduct (Variables|Default|GetPrevLookat) _returnvalue_2)))
        (Default|CallOnPlayerTurnedQuickly)))
    (:then_1
      (Variables|Default|SetPrevLookat _returnvalue_2))))

(fn ConstructionScript)