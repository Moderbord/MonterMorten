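; MonsterMover is an effect that repeatedly sends a billboard sprite monster (a "moose") travelling along a spline.
; Each walk picks a random sprite, shows it, and plays a timeline at the set movement rate to move MooseDad along Spline1.
; A sine of distance travelled adds a vertical stride bob to the spline transform.
; On finish, the sprite hides and the walk restarts after a random delay.
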(event Custom|MooseWalk
  (bind _spline1 (Variables|Default|GetSpline1))
  (Rendering|Components|Sprite|SetSprite (Variables|Default|GetBillboard) (.OutItem (Utilities|Array|Random (Variables|Default|GetSprites))))
  (Rendering|SetVisibility (Variables|Default|GetBillboard) true true)
  (Components|Timeline|SetPlayRate (Variables|Default|GetSplineMover) (Variables|Default|GetMovementRate))
  (bind _move_track (Timeline|SplineMover Play)
    (:Update
      (Transformation|SetWorldTransform (Variables|Default|GetMooseDad) (Math|Transform|MakeTransform (+ (* (Math|Vector|MakeVector 0.0 0.0 (Variables|Default|GetStrideHeight)) (Math|Trig|Sin(Radians) (* (Variables|Default|GetStride) (* (Spline|GetSplineLength _spline1) _move_track)))) (.Location (Math|Transform|BreakTransform (Spline|GetTransformatDistanceAlongSpline _spline1 (* (Spline|GetSplineLength _spline1) _move_track) "World" true)))) (.Rotation (Math|Transform|BreakTransform (Spline|GetTransformatDistanceAlongSpline _spline1 (* (Spline|GetSplineLength _spline1) _move_track) "World" true))) (.Scale (Math|Transform|BreakTransform (Spline|GetTransformatDistanceAlongSpline _spline1 (* (Spline|GetSplineLength _spline1) _move_track) "World" true)))) false false))
    (:Finished
      (Rendering|SetVisibility (Variables|Default|GetBillboard) false true)
      (Utilities|FlowControl|Delay (Math|Random|RandomFloatinRange (Variables|Default|GetMinMooseDelay) (Variables|Default|GetMaxMooseDelay)))
      (CallFunction|MooseWalk))))

(event EventBeginPlay
  (CallFunction|MooseWalk))

(fn ConstructionScript)