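; Orbiter is an actor Blueprint that moves along a curving path by stepping sideways and turning every tick.
; Each Tick offsets its world location along its right vector by Speed times Range, then adds Speed to its yaw, writing both results as relative transforms.
; The motion is not scaled by delta time.
; BeginPlay stores the owner in Parent, which the graph never reads.
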(event EventBeginPlay
  (Variables|Default|SetParent (Components|GetOwner)))

(event Collision|EventActorBeginOverlap
  (params (OtherActor :type Actor%20Object%20Reference)))

(event EventTick
  (params (DeltaSeconds :type Float%20%28single-precision%29))
  (bind _returnvalue (Transformation|GetActorRotation))
  (Utilities|FlowControl|Sequence
    (:then_0
      (Transformation|SetActorRelativeLocation (+ (* (* (Transformation|GetActorRightVector) (Variables|Default|GetSpeed)) (Variables|Default|GetRange)) (Transformation|GetActorLocation))))
    (:then_1
      (Transformation|SetActorRelativeRotation (Math|Rotator|MakeRotator (.roll _returnvalue) (.pitch _returnvalue) (+ (.yaw _returnvalue) (Variables|Default|GetSpeed)))))))

(fn ConstructionScript)