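; Lantern actor that sways with the wind and reports whether the player is inside its light.
; Each tick it syncs the point light's attenuation and the SpookRadius sphere to LightRadius.
; While movement is allowed, Blow repeatedly eases the mesh by the first WeatherController's wind direction and yaw over random durations, pausing between moves.
; Any overlap starting or ending on the sphere sets OutsideLight and broadcasts OnPlayerInLightChanged, without filtering for the player.
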(event OnComponentEndOverlap(SpookRadius)
  (params (OverlappedComponent :type Primitive%20Component%20Object%20Reference) (OtherActor :type Actor%20Object%20Reference) (OtherComp :type Primitive%20Component%20Object%20Reference) (OtherBodyIndex :type Integer))
  (Variables|Default|SetOutsideLight true)
  (Default|CallOnPlayerinLightChanged (Variables|Default|GetOutsideLight)))

(event OnComponentBeginOverlap(SpookRadius)
  (params (OverlappedComponent :type Primitive%20Component%20Object%20Reference) (OtherActor :type Actor%20Object%20Reference) (OtherComp :type Primitive%20Component%20Object%20Reference) (OtherBodyIndex :type Integer) (bFromSweep :type Boolean) (SweepResult :type Hit%20Result%20Structure%20%28by%20ref%29))
  (Variables|Default|SetOutsideLight false)
  (Default|CallOnPlayerinLightChanged (Variables|Default|GetOutsideLight)))

(event Custom|Blow
  (bind _lanternmesh (Variables|Default|GetLanternMesh))
  (bind _relativelocation (Variables|/Script/Engine.SceneComponent|GetRelativeLocation _lanternmesh))
  (bind _outactors (Actor|GetAllActorsOfClass "/Game/Blueprints/Weather/WeatherController.WeatherController_C"))
  (if (Variables|Default|GetAllowMovement)
    (Components|MoveComponentTo _lanternmesh (Math|Vector|MakeVector (+ (.x _relativelocation) (.x (Variables|/Game/Blueprints/Weather/WeatherController.WeatherController_C|GetWindDirection (Utilities|Array|Get(acopy) _outactors)))) (+ (.y _relativelocation) (.y (Variables|/Game/Blueprints/Weather/WeatherController.WeatherController_C|GetWindDirection (Utilities|Array|Get(acopy) _outactors)))) (.z _relativelocation)) (Math|Rotator|MakeRotator 0.0 0.0 (+ (.yaw (Variables|/Script/Engine.SceneComponent|GetRelativeRotation _lanternmesh)) (.yaw (Variables|/Game/Blueprints/Weather/WeatherController.WeatherController_C|GetLanternRotation (Utilities|Array|Get(acopy) _outactors))))) false false (Math|Random|RandomFloatinRange 1e+01 18.0) false :!label _label)
    (Utilities|FlowControl|Delay (Variables|Default|GetForcedWindDelay))
    (CallFunction|Blow)
    (else
      (goto _label Stop))))

(event EventBeginPlay
  (bind _lightradius (Variables|Default|GetLightRadius))
  (Rendering|Lighting|SetAttenuationRadius (Variables|Default|GetPointLight) _lightradius)
  (Components|Sphere|SetSphereRadius (Variables|Default|GetSpookRadius) _lightradius true)
  (CallFunction|Blow))

(event EventTick
  (params (DeltaSeconds :type Float%20%28single-precision%29))
  (bind _lightradius (Variables|Default|GetLightRadius))
  (Rendering|Lighting|SetAttenuationRadius (Variables|Default|GetPointLight) _lightradius)
  (Components|Sphere|SetSphereRadius (Variables|Default|GetSpookRadius) _lightradius true))

(fn ConstructionScript)