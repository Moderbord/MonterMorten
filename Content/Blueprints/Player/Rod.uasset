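; Player fishing rod Blueprint with a cable, a spinning cylinder that acts as a reel, and a physics-constrained line.
; Unconnected logic attaches the cable end, then a timeline spins the cylinder while shrinking the constraint's linear limits to reel in.
; A separate unconnected node pushes the Bajsfisk component toward the rod with a force.
; BeginPlay, GetNapp and NappEnd are empty, so none of this logic runs.
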(event Custom|GetNapp)

(event Custom|NappEnd)

(event EventBeginPlay)

(fn ConstructionScript)