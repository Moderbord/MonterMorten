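; Drill actor that animates its bit spinning and descending once play begins, with no interaction logic in its graph.
; BeginPlay stores the world location of DrillSeparateCube and plays a timeline from the start.
; One timeline track drives both lerps: DrillSeparateCube003 rotates through ten full turns in relative space while DrillSeparateCube moves straight down in world space without sweep.
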(event EventBeginPlay
  (Variables|Default|SetStoreWL (Transformation|GetWorldLocation (Variables|Default|Getdrill_separate_Cube)))
  (bind _newtrack_0 (Timeline|Timeline_0 PlayFromStart)
    (:Update
      (Transformation|SetRelativeRotation (Variables|Default|Getdrill_separate_Cube_003) (Math|Rotator|Lerp(Rotator) "0, 0, 0" "0,-3600.000000, 0" _newtrack_0) false false)
      (Transformation|SetWorldLocation (Variables|Default|Getdrill_separate_Cube) (Math|Vector|Lerp(Vector) (Variables|Default|GetStoreWL) (- (Variables|Default|GetStoreWL) "0, 0,120.000000") _newtrack_0) false false))))

(fn ConstructionScript)