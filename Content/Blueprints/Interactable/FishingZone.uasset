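; FishingZone is an interactable area that tells the first-person character when it is inside and hosts the fishing hole's drill and chair.
; Overlap events set the zone reference and inside flag on the character.
; SpawnChair places an attached chair with its camera facing the collision point, and PanCamera moves the player's view to it.
; SpawnDrill attaches a drill there with a downward camera matching the player's yaw, while DespawnDrill removes it.
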(event Custom|SpawnChair
  (params (Location :type Vector))
  ;[1 1 1] Spawn chair and set char camera to look at hole
  (Variables|Default|SetHasChair true)
  (bind _returnvalue (Game|SpawnActorfromClass "/Game/Blueprints/Interactable/Chair.Chair_C" (Math|Transform|MakeTransform Location (Math|Rotator|FindLookatRotation Location (Transformation|GetWorldLocation (Variables|Default|GetCollision)))) "Undefined" 0 0))
  (bind _output_get (Variables|Default|SetChair _returnvalue))
  (Transformation|SetWorldRotation (Variables|/Game/Blueprints/Interactable/Chair.Chair_C|GetCamera _output_get) (Math|Rotator|FindLookatRotation (Transformation|GetWorldLocation (Variables|/Game/Blueprints/Interactable/Chair.Chair_C|GetCamera _output_get)) (Transformation|GetWorldLocation (Variables|Default|GetCollision))) false false)
  (Transformation|AttachActorToActor _output_get self "None" "KeepWorld" "KeepWorld" "KeepWorld" true))

(event Custom|PanCamera
  ;[1 1 1] Pan camera to char camera
  (bind _asfirst_person_character (Utilities|Casting|CastToFirstPersonCharacter (Game|Player|GetPlayerPawn 0)))
  (Default|PanCamera _asfirst_person_character (Transformation|GetWorldTransform (Variables|/Game/Blueprints/Interactable/Chair.Chair_C|GetCamera (Variables|Default|GetChair)))))

(event EventBeginPlay)

(event Collision|EventActorBeginOverlap
  (params (OtherActor :type Actor%20Object%20Reference))
  ;[1 1 1] checks if character is in or out of zone
  (bind _asfirst_person_character (Utilities|Casting|CastToFirstPersonCharacter OtherActor))
  (Default|SetFishingZone _asfirst_person_character self)
  (Variables|/Game/FirstPersonBP/Blueprints/FirstPersonCharacter.FirstPersonCharacter_C|SetInsideFishingZone _asfirst_person_character true))

(event EventTick
  (params (DeltaSeconds :type Float%20%28single-precision%29)))

(event Collision|EventActorEndOverlap
  (params (OtherActor :type Actor%20Object%20Reference))
  ;[1 1 1] checks if character is in or out of zone
  (bind _asfirst_person_character (Utilities|Casting|CastToFirstPersonCharacter OtherActor))
  (Default|SetFishingZone _asfirst_person_character self)
  (Variables|/Game/FirstPersonBP/Blueprints/FirstPersonCharacter.FirstPersonCharacter_C|SetInsideFishingZone _asfirst_person_character false))

(fn ConstructionScript)

(fn SpawnDrill
  (bind _returnvalue (Game|SpawnActorfromClass "/Game/Blueprints/Interactable/Drill.Drill_C" (Math|Conversions|ToTransform(Vector) (Transformation|GetWorldLocation (Variables|Default|GetCollision))) "Undefined" 0 0))
  (Variables|Default|SetDrill _returnvalue)
  (Transformation|AttachActorToActor _returnvalue self "None" "KeepWorld" "KeepWorld" "KeepWorld" true)
  (bind _asfirst_person_character (Utilities|Casting|CastToFirstPersonCharacter (Game|Player|GetPlayerPawn 0)))
  (Transformation|SetWorldRotation (Variables|/Game/Blueprints/Interactable/Drill.Drill_C|GetCamera _returnvalue) (Math|Rotator|MakeRotator (.Roll (Math|Rotator|BreakRotator (Transformation|GetWorldRotation (Variables|/Script/Engine.Character|GetMesh _asfirst_person_character)))) -9e+01 (.Yaw (Math|Rotator|BreakRotator (Transformation|GetWorldRotation (Variables|/Script/Engine.Character|GetMesh _asfirst_person_character))))) false false)
  (return _returnvalue))

(fn DespawnDrill
  (bind _drill (Variables|Default|GetDrill))
  (Transformation|DetachFromActor _drill "KeepWorld" "KeepWorld" "KeepWorld")
  (Actor|DestroyActor _drill))